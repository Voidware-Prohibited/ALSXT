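; ALSXT AI spline character that randomizes its appearance and combat posture and switches to its KillerCamera on play.
; The construction script builds a per-body-part color map from clothing and skin palettes, rolling each part independently.
; Looping timers re-randomize combat stance, weapon readiness, rotation mode and aiming, and match camera focal length and focus to spring arm length.
; A timeline sweeps the look-at target's offset; overlay switching is disconnected.
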(event Custom|SetFocusDistance
  (bind _killercamera (Variables|Default|GetKillerCamera))
  (bind _killerspringarm (Variables|Default|GetKillerSpringArm))
  (bind _targetarmlength (Variables|/Script/Engine.SpringArmComponent|GetTargetArmLength _killerspringarm))
  (Variables|/Script/CinematicCamera.CineCameraComponent|SetCurrentFocalLength _killercamera (- (* _targetarmlength 0.1) 1e+01))
  (Utilities|Struct|SetmembersinCameraFocusSettings (Variables|/Script/CinematicCamera.CineCameraComponent|GetFocusSettings _killercamera) (+ _targetarmlength 215.0)))

(event Custom|Move%20Look%20At%20Target
  (bind _lr (Timeline|Look%20At%20Target%20Movement%20Timeline Play)
    (:Update
      (Variables|Default|SetLR _lr)
      (Variables|/Script/Engine.SpringArmComponent|SetTargetOffset (Variables|Default|GetLookAtTargetSpringArm) (Math|Vector|MakeVector 0.0 (Math|Float|Lerp -1e+03 1e+03 (Variables|Default|GetLR)) (Math|Float|Lerp 0.0 6e+02 (Variables|Default|GetLR)))))))

(event EventBeginPlay
  (|CallParentFunction)
  (Utilities|Time|SetTimerbyFunctionName 0 "SetFocusDistance" 0.1 true)
  (Utilities|Time|SetTimerbyFunctionName 0 "SetOverlayandStances" 3.0 true)
  (Components|Activation|Deactivate (Variables|Default|GetCamera))
  (Components|Activation|Activate (Variables|Default|GetKillerCamera) true)
  (CallFunction|MoveLookatTarget))

(fn ConstructionScript
  (bind _returnvalue (Math|Random|RandomIntegerinRange 0 4))
  (bind _returnvalue_2 (Math|Random|RandomBoolwithWeight 0.2))
  (bind _returnvalue_3 (Math|Random|RandomBool))
  (bind _returnvalue_4 (Math|Random|RandomIntegerinRange 0 3))
  (bind _returnvalue_5 (Math|Random|RandomIntegerinRange 0 1))
  (bind _returnvalue_6 (Math|Random|RandomIntegerinRange 0 7))
  (bind _returnvalue_7 (Math|Random|RandomIntegerinRange 0 3))
  (bind _returnvalue_8 (Utilities|Select :Index _returnvalue_4 :Option%200 "(R=0.541176,G=0.317647,B=0.258824,A=1.000000)" :Option%201 "(R=0.812500,G=0.476902,B=0.388587,A=1.000000)" :Option%202 "(R=0.260417,G=0.152853,B=0.124547,A=1.000000)" :Option%203 "(R=0.041667,G=0.021626,B=0.011035,A=1.000000)"))
  (bind _returnvalue_9 (Utilities|Select :Index _returnvalue_5 :Option%200 "" :Option%201 "(R=0.218750,G=0.113538,B=0.057932,A=1.000000)"))
  (bind _returnvalue_10 (Utilities|Select :Index _returnvalue :Option%200 "(R=0.015686,G=0.015686,B=0.015686,A=1.000000)" :Option%201 "(R=1.000000,G=1.000000,B=1.000000,A=1.000000)" :Option%202 "(R=0.218750,G=0.113538,B=0.057932,A=1.000000)" :Option%203 "(R=0.000000,G=0.180420,B=1.000000,A=1.000000)" :Option%204 "(R=1.000000,G=0.000000,B=0.000000,A=1.000000)"))
  (bind _returnvalue_11 (Utilities|Select :Index _returnvalue_6 :Option%200 "(R=1.000000,G=1.000000,B=1.000000,A=1.000000)" :Option%201 "(R=0.062745,G=0.062745,B=0.062745,A=1.000000)" :Option%202 "(R=0.200000,G=0.200000,B=1.000000,A=1.000000)" :Option%203 "(R=1.000000,G=0.000000,B=0.022732,A=1.000000)" :Option%204 "(R=0.098039,G=0.121569,B=0.019608,A=1.000000)" :Option%205 "(R=1.000000,G=0.751139,B=0.130208,A=1.000000)" :Option%206 "(R=1.000000,G=0.343750,B=0.843971,A=1.000000)" :Option%207 "(R=0.162145,G=0.000000,B=0.369792,A=1.000000)"))
  (bind _returnvalue_12 (Utilities|Select :Index _returnvalue_7 :Option%200 "" :Option%201 "(R=0.098039,G=0.121569,B=0.019608,A=1.000000)" :Option%202 "(R=0.007499,G=0.116971,B=0.508881,A=1.000000)" :Option%203 "(R=1.000000,G=1.000000,B=1.000000,A=1.000000)"))
  (bind _returnvalue_13 (select _returnvalue_2 _returnvalue_9 _returnvalue_8))
  (bind _returnvalue_14 (select _returnvalue_3 _returnvalue_11 _returnvalue_8))
  (Variables|Default|SetALSXT_MeshMaterialColors (Utilities|Map|MakeMap "Pelvis" _returnvalue_12 "Torso" _returnvalue_11 "UpperArmL" _returnvalue_11 "ShoulderL" _returnvalue_11 "LowerArmL" _returnvalue_14 "Thighs" _returnvalue_12 "LowerLegs" (select (Math|Random|RandomBoolwithWeight 0.15) _returnvalue_10 (select (Math|Random|RandomBool) _returnvalue_8 _returnvalue_12)) "Feet" _returnvalue_10 "HandL" _returnvalue_13 "UpperArmR" _returnvalue_11 "ShoulderR" _returnvalue_11 "LowerArmR" _returnvalue_14 "HandR" _returnvalue_13 "Head" _returnvalue_8))
  (|CallParentFunction))

(fn SetOverlayandStances
  (bind _returnvalue (Math|Random|RandomBool))
  (Class|ALSXTCharacter|SetDesiredCombatStance (select _returnvalue (GameplayTags|MakeLiteralGameplayTag "(TagName=\"Als.Combat Stance.Aiming\")") (GameplayTags|MakeLiteralGameplayTag "(TagName=\"Als.Combat Stance.Ready\")")))
  (Class|ALSXTCharacter|SetDesiredWeaponReadyPosition (select _returnvalue (GameplayTags|MakeLiteralGameplayTag "(TagName=\"Als.Weapon Ready Position.Aiming\")") (GameplayTags|MakeLiteralGameplayTag "(TagName=\"Als.Weapon Ready Position.Low Ready\")")))
  (Class|AlsCharacter|SetDesiredRotationMode (select _returnvalue (GameplayTags|MakeLiteralGameplayTag "(TagName=\"Als.RotationMode.Aiming\")") (GameplayTags|MakeLiteralGameplayTag "(TagName=\"Als.RotationMode.LookingDirection\")")))
  (Class|AlsCharacter|SetDesiredAiming _returnvalue)
  (return))