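; ALSXT AI character that randomizes its look and can cycle through animation overlays and stances.
; The construction script fills a per-body-region color map from random skin and clothing palettes, with chance rolls for bare skin, gloves or tall boots, before calling the parent script.
; On possession, an optional looping timer randomizes overlay mode, combat stance and aiming while status is Normal.
; GetStamina returns a fixed half value.
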(event EventBeginPlay
  (|CallParentFunction))

(event EventPossessed
  (params (NewController :type Controller%20Object%20Reference))
  (|CallParentFunction NewController)
  (if (Variables|Default|GetEnableOverlayAndStanceCycling)
    (Utilities|Time|SetTimerbyFunctionName 0 "SetOverlayandStances" 3e+01 true)))

(fn ConstructionScript
  (bind _returnvalue (Math|Random|RandomIntegerinRange 0 4))
  (bind _returnvalue_2 (Math|Random|RandomBoolwithWeight 0.2))
  (bind _returnvalue_3 (Math|Random|RandomBool))
  (bind _returnvalue_4 (Math|Random|RandomIntegerinRange 0 3))
  (bind _returnvalue_5 (Math|Random|RandomIntegerinRange 0 1))
  (bind _returnvalue_6 (Math|Random|RandomIntegerinRange 0 7))
  (bind _returnvalue_7 (Math|Random|RandomIntegerinRange 0 3))
  (bind _returnvalue_8 (Utilities|Select :Index _returnvalue_4 :Option%200 "(R=0.541176,G=0.317647,B=0.258824,A=1.000000)" :Option%201 "(R=0.812500,G=0.476902,B=0.388587,A=1.000000)" :Option%202 "(R=0.260417,G=0.152853,B=0.124547,A=1.000000)" :Option%203 "(R=0.041667,G=0.021626,B=0.011035,A=1.000000)"))
  (bind _returnvalue_9 (Utilities|Select :Index _returnvalue_5 :Option%200 "" :Option%201 "(R=0.218750,G=0.113538,B=0.057932,A=1.000000)"))
  (bind _returnvalue_10 (Utilities|Select :Index _returnvalue :Option%200 "(R=0.015686,G=0.015686,B=0.015686,A=1.000000)" :Option%201 "(R=1.000000,G=1.000000,B=1.000000,A=1.000000)" :Option%202 "(R=0.218750,G=0.113538,B=0.057932,A=1.000000)" :Option%203 "(R=0.000000,G=0.180420,B=1.000000,A=1.000000)" :Option%204 "(R=1.000000,G=0.000000,B=0.000000,A=1.000000)"))
  (bind _returnvalue_11 (Utilities|Select :Index _returnvalue_6 :Option%200 "(R=1.000000,G=1.000000,B=1.000000,A=1.000000)" :Option%201 "(R=0.062745,G=0.062745,B=0.062745,A=1.000000)" :Option%202 "(R=0.200000,G=0.200000,B=1.000000,A=1.000000)" :Option%203 "(R=1.000000,G=0.000000,B=0.022732,A=1.000000)" :Option%204 "(R=0.098039,G=0.121569,B=0.019608,A=1.000000)" :Option%205 "(R=1.000000,G=0.751139,B=0.130208,A=1.000000)" :Option%206 "(R=1.000000,G=0.343750,B=0.843971,A=1.000000)" :Option%207 "(R=0.162145,G=0.000000,B=0.369792,A=1.000000)"))
  (bind _returnvalue_12 (Utilities|Select :Index _returnvalue_7 :Option%200 "" :Option%201 "(R=0.098039,G=0.121569,B=0.019608,A=1.000000)" :Option%202 "(R=0.007499,G=0.116971,B=0.508881,A=1.000000)" :Option%203 "(R=1.000000,G=1.000000,B=1.000000,A=1.000000)"))
  (bind _returnvalue_13 (select _returnvalue_2 _returnvalue_9 _returnvalue_8))
  (bind _returnvalue_14 (select _returnvalue_3 _returnvalue_11 _returnvalue_8))
  (Variables|Default|SetALSXT_MeshMaterialColors (Utilities|Map|MakeMap "Pelvis" _returnvalue_12 "Torso" _returnvalue_11 "UpperArmL" _returnvalue_11 "ShoulderL" _returnvalue_11 "LowerArmL" _returnvalue_14 "Thighs" _returnvalue_12 "LowerLegs" (select (Math|Random|RandomBoolwithWeight 0.15) _returnvalue_10 (select (Math|Random|RandomBool) _returnvalue_8 _returnvalue_12)) "Feet" _returnvalue_10 "HandL" _returnvalue_13 "UpperArmR" _returnvalue_11 "ShoulderR" _returnvalue_11 "LowerArmR" _returnvalue_14 "HandR" _returnvalue_13 "Head" _returnvalue_8))
  (|CallParentFunction))

(fn SetOverlayandStances
  (bind _array (Utilities|Array|MakeArray "(TagName=\"Als.OverlayMode.Axe One Handed\")" "(TagName=\"Als.OverlayMode.Barrel\")" "(TagName=\"Als.OverlayMode.Binoculars\")" "(TagName=\"Als.OverlayMode.Bow\")" "(TagName=\"Als.OverlayMode.Feminine\")" "(TagName=\"Als.OverlayMode.HandsTied\")" "(TagName=\"Als.OverlayMode.Injured\")" "(TagName=\"Als.OverlayMode.Knife\")" "(TagName=\"Als.OverlayMode.M4\")" "(TagName=\"Als.OverlayMode.PistolTwoHanded\")" "(TagName=\"Als.OverlayMode.Torch\")" "(TagName=\"Als.OverlayMode.PistolOneHanded\")"))
  (if (== (Class|ALSXTCharacter|GetDesiredStatus) "(TagName=\"Als.Status.Normal\")")
    (Class|AlsCharacter|SetOverlayMode (Utilities|Array|Get(acopy) _array (Math|Random|RandomIntegerinRange 0 (Utilities|Array|LastIndex _array))))
    (Class|ALSXTCharacter|SetDesiredCombatStance (select (Math|Random|RandomBool) (GameplayTags|MakeLiteralGameplayTag "(TagName=\"Als.Combat Stance.Ready\")") (GameplayTags|MakeLiteralGameplayTag "(TagName=\"Als.Combat Stance.Neutral\")")))
    (Class|AlsCharacter|SetDesiredAiming (Math|Random|RandomBool))
    (return)))

(fn GetStamina
  (return 0.5))