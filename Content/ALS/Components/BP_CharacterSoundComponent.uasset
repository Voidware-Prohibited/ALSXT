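; Character component that plays action, attack, damage and death vocalizations for its owning Character, reacting to OnTakeAnyDamage for hurt sounds.
; Authority switches route calls through Server and Multi events, which spawn MetaSounds at the mesh's voice socket.
; Each sets sex, variant, stamina and health parameters, mostly placeholders, and reports a noise event.
; The alive check is stubbed true, so the damage Multi event always plays the death sound.
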(event Custom|Character%20Action%20Sound
  (Networking|SwitchHasAuthority
    (:Authority
      (CallFunction|CharacterActionSoundMulti))
    (:Remote
      (CallFunction|CharacterActionSoundServer))))

(event Custom|Character%20Attack%20Sound
  (Networking|SwitchHasAuthority
    (:Authority
      (CallFunction|CharacterAttackSoundServer))
    (:Remote
      (CallFunction|CharacterAttackSoundMulti))))

(event Custom|Character%20Damage%20Sound%20Multi
  (params (Damage :type Float%20%28double-precision%29) (Damage%20Type :type Damage%20Type%20Object%20Reference) (Damage%20Causer :type Actor%20Object%20Reference))
  (bind _debug_mode (Variables|Settings|GetDebug%20Mode))
  (bind _mesh (Variables|Default|GetMesh))
  (bind _voice_socket_name (Variables|Settings|GetVoice%20Socket%20Name))
  (bind _returnvalue (Transformation|GetSocketLocation _mesh _voice_socket_name))
  (Development|PrintString "Damage Sound" _debug_mode _debug_mode)
  (if true ; Check if Alive
    (CallFunction|CharacterDeathSoundMulti Damage Damage%20Type Damage%20Causer)
    (else
      (bind _returnvalue_2 (Audio|SpawnSoundAttached "/ALSXT/ALS/Audio/Character/MSS_CharacterDamage.MSS_CharacterDamage" _mesh (Variables|Settings|GetVoice%20Socket%20Name) _returnvalue (Math|Rotator|MakeRotfromX (Math|Vector|GetForwardVector _mesh)) "KeepRelativeOffset" false 1.0 1.0 0.0 0 0))
      (bind _output_get (Variables|Default|SetDamage%20Sound _returnvalue_2))
      (Utilities|IsValid _output_get :!label _label
        (:Is%20Valid
          (Effects|Components|ParticleSystem|SetIntParameter _output_get "Sex" 1)
          (Effects|Components|ParticleSystem|SetIntParameter _output_get "Variant" 1)
          (Audio|Parameter|SetFloatParameter _output_get "Stamina" 1.0 :!class /Script/Engine.AudioComponent)
          (Audio|Parameter|SetFloatParameter _output_get "Health" 1.0 :!class /Script/Engine.AudioComponent)
          (Audio|Components|Audio|Play _output_get 0.0)
          (Class|AISenseHearing|ReportNoiseEvent _returnvalue 1.0 (Components|GetOwner) (Variables|Settings|NoiseEvent|GetVocalization%20Noise%20Event%20Max%20Range) (Variables|Settings|NoiseEvent|GetVocalization%20Noise%20Event%20Tag)))
        (:Is%20Not%20Valid
          (Utilities|FlowControl|Delay 0.2)
          (goto _label))))))

(event Custom|Character%20Death%20Sound%20Event
  (bind _debug_mode (Variables|Settings|GetDebug%20Mode))
  (bind _mesh (Variables|Default|GetMesh))
  (bind _voice_socket_name (Variables|Settings|GetVoice%20Socket%20Name))
  (bind _returnvalue (Transformation|GetSocketLocation _mesh _voice_socket_name))
  (Development|PrintString "Death Sound" _debug_mode _debug_mode)
  (bind _returnvalue_2 (Audio|SpawnSoundAttached "/ALSXT/ALS/Audio/Character/MSS_CharacterDeath.MSS_CharacterDeath" _mesh (Variables|Settings|GetVoice%20Socket%20Name) _returnvalue (Math|Rotator|MakeRotfromX (Math|Vector|GetForwardVector _mesh)) "KeepRelativeOffset" false 1.0 1.0 0.0 0 0))
  (bind _output_get (Variables|Default|SetDeath%20Sound _returnvalue_2))
  (Utilities|IsValid _output_get :!label _label
    (:Is%20Valid
      (Effects|Components|ParticleSystem|SetIntParameter _output_get "Sex" (Utilities|Select :Index (Variables|DoNotEdit|GetDesired%20Sex) :Option%200 0 :Option%201 0))
      (Effects|Components|ParticleSystem|SetIntParameter _output_get "Variant" (Utilities|Select :Index (Variables|Settings|GetVoiceVariant) :NewEnumerator0 1 :NewEnumerator1 2 :NewEnumerator2 3))
      (Audio|Parameter|SetFloatParameter _output_get "Stamina" 0.0 :!class /Script/Engine.AudioComponent)
      (Audio|Parameter|SetFloatParameter _output_get "Health" 0.0 :!class /Script/Engine.AudioComponent)
      (Audio|Components|Audio|Play _output_get 0.0)
      (Class|AISenseHearing|ReportNoiseEvent _returnvalue 1.0 (Components|GetOwner) (Variables|Settings|NoiseEvent|GetDeath%20Noise%20Event%20Max%20Range) (Variables|Settings|NoiseEvent|GetVocalization%20Noise%20Event%20Tag)))
    (:Is%20Not%20Valid
      (Utilities|FlowControl|Delay 0.2)
      (goto _label))))

(event Custom|Character%20Attack%20Sound%20Server
  (CallFunction|CharacterAttackSoundMulti))

(event Custom|Character%20Attack%20Sound%20Multi
  (CallFunction|CharacterAttackSoundEvent))

(event Custom|Character%20Death%20Sound
  (params (Damage :type Float%20%28double-precision%29) (Damage%20Type :type Damage%20Type%20Object%20Reference) (Damage%20Causer :type Actor%20Object%20Reference))
  (Networking|SwitchHasAuthority
    (:Authority
      (CallFunction|CharacterDeathSoundServer Damage Damage%20Type Damage%20Causer))
    (:Remote
      (CallFunction|CharacterDeathSoundMulti Damage Damage%20Type Damage%20Causer))))

(event Custom|Character%20Damage%20Sound%20Server
  (params (Damage :type Float%20%28double-precision%29) (Damage%20Type :type Damage%20Type%20Object%20Reference) (Damage%20Causer :type Actor%20Object%20Reference))
  (CallFunction|CharacterDamageSoundMulti Damage Damage%20Type Damage%20Causer))

(event Custom|Character%20Damage%20Sound
  (params (Damage :type Float%20%28double-precision%29) (Damage%20Type :type Damage%20Type%20Object%20Reference) (Damage%20Causer :type Actor%20Object%20Reference))
  (if (<= 0.0 0.0)
    (CallFunction|CharacterDeathSound Damage Damage%20Type Damage%20Causer)
    (else
      (Networking|SwitchHasAuthority
        (:Authority
          (CallFunction|CharacterDamageSoundServer Damage Damage%20Type Damage%20Causer))
        (:Remote
          (CallFunction|CharacterDamageSoundMulti Damage Damage%20Type Damage%20Causer))))))

(event Custom|Character%20Action%20Sound%20Server
  (CallFunction|CharacterActionSoundMulti))

(event Custom|OnTakeAnyDamage_Event
  (params (DamagedActor :type Actor%20Object%20Reference) (Damage :type Float%20%28single-precision%29) (DamageType :type Damage%20Type%20Object%20Reference) (InstigatedBy :type Controller%20Object%20Reference) (DamageCauser :type Actor%20Object%20Reference))
  (CallFunction|CharacterDamageSound Damage DamageType DamageCauser))

(event Custom|Character%20Action%20Sound%20Multi
  (bind _debug_mode (Variables|Settings|GetDebug%20Mode))
  (bind _mesh (Variables|Default|GetMesh))
  (bind _voice_socket_name (Variables|Settings|GetVoice%20Socket%20Name))
  (bind _returnvalue (Transformation|GetSocketLocation _mesh _voice_socket_name))
  (Development|PrintString "Action Sound" _debug_mode _debug_mode)
  (bind _returnvalue_2 (Audio|SpawnSoundAttached "/ALSXT/ALS/Audio/Character/MSS_CharacterAction.MSS_CharacterAction" _mesh (Variables|Settings|GetVoice%20Socket%20Name) _returnvalue (Math|Rotator|MakeRotfromX (Math|Vector|GetForwardVector _mesh)) "KeepRelativeOffset" false 1.0 1.0 0.0 0 0))
  (bind _output_get (Variables|Default|SetAction%20Sound _returnvalue_2))
  (Utilities|IsValid _output_get :!label _label
    (:Is%20Valid
      (Effects|Components|ParticleSystem|SetIntParameter _output_get "Sex" (Utilities|Select :Index 0 :Option%200 1 :Option%201 2))
      (Effects|Components|ParticleSystem|SetIntParameter _output_get "Variant" 1)
      (Audio|Parameter|SetFloatParameter _output_get "Stamina" 5e+01 :!class /Script/Engine.AudioComponent)
      (Audio|Parameter|SetFloatParameter _output_get "Health" 1e+02 :!class /Script/Engine.AudioComponent)
      (Audio|Components|Audio|Play _output_get 0.0)
      (Class|AISenseHearing|ReportNoiseEvent _returnvalue 1.0 (Components|GetOwner) (Variables|Settings|NoiseEvent|GetVocalization%20Noise%20Event%20Max%20Range) (Variables|Settings|NoiseEvent|GetVocalization%20Noise%20Event%20Tag)))
    (:Is%20Not%20Valid
      (Utilities|FlowControl|Delay 0.2)
      (goto _label))))

(event Custom|Character%20Attack%20Sound%20Event
  (bind _mesh (Variables|Default|GetMesh))
  (bind _voice_socket_name (Variables|Settings|GetVoice%20Socket%20Name))
  (bind _debug_mode (Variables|Settings|GetDebug%20Mode))
  (bind _returnvalue (Transformation|GetSocketLocation _mesh _voice_socket_name))
  (Development|PrintString "Attack Sound" _debug_mode _debug_mode)
  (bind _returnvalue_2 (Audio|SpawnSoundAttached "/ALSXT/ALS/Audio/Character/MSS_CharacterAction.MSS_CharacterAction" _mesh (Variables|Settings|GetVoice%20Socket%20Name) _returnvalue (Math|Rotator|MakeRotfromX (Math|Vector|GetForwardVector _mesh)) "KeepRelativeOffset" false 1.0 1.0 0.0 0 0))
  (bind _output_get (Variables|Default|SetAttack%20Sound _returnvalue_2))
  (Utilities|IsValid _output_get :!label _label
    (:Is%20Valid
      (Effects|Components|ParticleSystem|SetIntParameter _output_get "Sex" (Utilities|Select :Index (Variables|DoNotEdit|GetDesired%20Sex) :Option%200 0 :Option%201 0))
      (Effects|Components|ParticleSystem|SetIntParameter _output_get "Variant" (Utilities|Select :Index (Variables|Settings|GetVoiceVariant) :NewEnumerator0 1 :NewEnumerator1 2 :NewEnumerator2 3))
      (Audio|Parameter|SetFloatParameter _output_get "Stamina" 0.0 :!class /Script/Engine.AudioComponent)
      (Audio|Parameter|SetFloatParameter _output_get "Health" 0.0 :!class /Script/Engine.AudioComponent)
      (Audio|Components|Audio|Play _output_get 0.0)
      (Class|AISenseHearing|ReportNoiseEvent _returnvalue 1.0 (Components|GetOwner) (Variables|Settings|NoiseEvent|GetVocalization%20Noise%20Event%20Max%20Range) (Variables|Settings|NoiseEvent|GetVocalization%20Noise%20Event%20Tag)))
    (:Is%20Not%20Valid
      (Utilities|FlowControl|Delay 0.2)
      (goto _label))))

(event Custom|Character%20Death%20Sound%20Server
  (params (Damage :type Float%20%28double-precision%29) (Damage%20Type :type Damage%20Type%20Object%20Reference) (Damage%20Causer :type Actor%20Object%20Reference))
  (CallFunction|CharacterDeathSoundMulti Damage Damage%20Type Damage%20Causer))

(event Custom|Character%20Death%20Sound%20Multi
  (params (Damage :type Float%20%28double-precision%29) (Damage%20Type :type Damage%20Type%20Object%20Reference) (Damage%20Causer :type Actor%20Object%20Reference))
  (CallFunction|CharacterDeathSoundEvent))

(event EventBeginPlay
  (bind _ascharacter (Utilities|Casting|CastToCharacter (Components|GetOwner)))
  (Variables|DoNotEdit|SetCharacter _ascharacter)
  (Variables|Default|SetMesh (Variables|/Script/Engine.Character|GetMesh (Variables|DoNotEdit|GetCharacter)))
  (Variables|DoNotEdit|SetDesired%20Sex 1)
  (EventDispatchers|AssignOnTakeAnyDamage (Variables|DoNotEdit|GetCharacter) (delegate Custom|OnTakeAnyDamage_Event)))

(event EventTick
  (params (DeltaSeconds :type Float%20%28single-precision%29)))