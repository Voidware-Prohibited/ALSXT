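; B_ImpactParticle is an impact particle actor that flies as a projectile and leaves a decal where it lands.
; Construction makes the Niagara component the one ProjectileMovement moves and randomizes its initial speed.
; A capsule hit on a StaticMeshActor spawns a B_DecalActor just off the surface, aligned to the normal with random yaw.
; The particle then destroys itself, and the decal attaches to the hit component, keeping its world transform.
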(event OnComponentHit(Capsule)
  (params (HitComponent :type Primitive%20Component%20Object%20Reference) (OtherActor :type Actor%20Object%20Reference) (OtherComp :type Primitive%20Component%20Object%20Reference) (NormalImpulse :type Vector :default "0, 0, 0") (Hit :type Hit%20Result%20Structure%20%28by%20ref%29))
  (bind (_bblockinghit _binitialoverlap _time _distance _location _impactpoint _normal _impactnormal _physmat _hitactor _hitcomponent) (Collision|BreakHitResult Hit))
  (Utilities|Casting|CastToStaticMeshActor OtherActor)
  (bind _returnvalue (Game|SpawnActorfromClass "/ALSXT/ALS/Blueprints/Impact/B_DecalActor.B_DecalActor_C" (Math|Transform|MakeTransform (+ _impactpoint (* _normal 2.0)) (Math|Rotator|CombineRotators (Math|Rotator|MakeRotfromX _normal) (Math|Rotator|MakeRotator 0.0 9e+01 (Math|Random|RandomFloatinRange -1.8e+02 1.8e+02)))) "AlwaysSpawn" "MultiplyWithRoot" 0 0))
  (Components|DestroyComponent (Variables|Default|GetProjectileMovement))
  (Actor|DestroyActor)
  (Transformation|AttachComponentToComponent _returnvalue _hitcomponent "None" "KeepWorld" "KeepWorld" "KeepWorld" true))

(event OnComponentHit(Niagara)
  (params (HitComponent :type Primitive%20Component%20Object%20Reference) (OtherActor :type Actor%20Object%20Reference) (OtherComp :type Primitive%20Component%20Object%20Reference) (NormalImpulse :type Vector :default "0, 0, 0") (Hit :type Hit%20Result%20Structure%20%28by%20ref%29)))

(event EventBeginPlay)

(event Collision|EventActorBeginOverlap
  (params (OtherActor :type Actor%20Object%20Reference)))

(event EventTick
  (params (DeltaSeconds :type Float%20%28single-precision%29))
  (Class|MovementComponent|MoveUpdatedComponent (Variables|Default|GetProjectileMovement) "0, 0, 0" "0, 0, 0" true))

(fn ConstructionScript
  (Components|Movement|SetUpdatedComponent (Variables|Default|GetProjectileMovement) (Variables|Default|GetNiagara))
  (Variables|/Script/Engine.ProjectileMovementComponent|SetInitialSpeed (Variables|Default|GetProjectileMovement) (Math|Random|RandomFloatinRange 1e+02 2.5e+02)))