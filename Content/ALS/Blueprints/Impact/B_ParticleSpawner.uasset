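; B_ParticleSpawner is an actor that periodically spawns B_ImpactParticle actors while slowly rotating.
; BeginPlay starts two looping timers: one spawns a particle at its Arrow component's world transform, the other applies small world-rotation increments.
; The rotation uses a fast timer, with Tick left unused.
; A disconnected snippet for a random-strength forward force on a Capsule never runs.
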(event Custom|Spawn%20Particle
  (Game|SpawnActorfromClass "/ALSXT/ALS/Blueprints/Impact/B_ImpactParticle.B_ImpactParticle_C" (Transformation|GetWorldTransform (Variables|Default|GetArrow)) "Undefined" 0 0))

(event Custom|Rotate
  (Class|Actor|AddActorWorldRotation "0.000000,0.010000,0.000000"))

(event EventBeginPlay
  (Utilities|Time|SetTimerbyFunctionName 0 "Spawn Particle" 2.0 true)
  (Utilities|Time|SetTimerbyEvent (delegate Custom|Rotate) 0.01 true))

(event Collision|EventActorBeginOverlap
  (params (OtherActor :type Actor%20Object%20Reference)))

(event EventTick
  (params (DeltaSeconds :type Float%20%28single-precision%29)))

(fn ConstructionScript)