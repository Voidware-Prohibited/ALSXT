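; BP_Foliage is a foliage Blueprint that plays a vegetation rustle sound when moving actors brush through it.
; BeginPlay binds a component begin-overlap event, which spawns the sound at the sweep location if the other actor implements ALSXTCollisionInterface and exceeds a speed threshold.
; A similar end-overlap handler with a lower threshold plays at the actor's location, but its binding is never executed.
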(event Custom|OnComponentBeginOverlap_Event
  (params (OverlappedComponent :type Primitive%20Component%20Object%20Reference) (OtherActor :type Actor%20Object%20Reference) (OtherComp :type Primitive%20Component%20Object%20Reference) (OtherBodyIndex :type Integer) (bFromSweep :type Boolean) (SweepResult :type Hit%20Result%20Structure%20%28by%20ref%29))
  (if (and (Utilities|DoesObjectImplementInterface OtherActor "/Script/ALSXT.ALSXTCollisionInterface") (> (Math|Vector|VectorLength (Transformation|GetVelocity OtherActor)) 3e+02))
    (Audio|SpawnSoundatLocation "/ALSXT/ALS/Audio/Footsteps/MS_Als_Footstep_Vegetation.MS_Als_Footstep_Vegetation" (.Location (Collision|BreakHitResult SweepResult)) "0, 0, 0" 1.0 1.0 0.0 0 0)))

(event Custom|OnComponentEndOverlap_Event
  (params (OverlappedComponent :type Primitive%20Component%20Object%20Reference) (OtherActor :type Actor%20Object%20Reference) (OtherComp :type Primitive%20Component%20Object%20Reference) (OtherBodyIndex :type Integer))
  (if (and (Utilities|DoesObjectImplementInterface OtherActor "/Script/ALSXT.ALSXTCollisionInterface") (> (Math|Vector|VectorLength (Transformation|GetVelocity OtherActor)) 1e+02))
    (Audio|SpawnSoundatLocation "/ALSXT/ALS/Audio/Footsteps/MS_Als_Footstep_Vegetation.MS_Als_Footstep_Vegetation" (Transformation|GetActorLocation OtherActor) "0, 0, 0" 1.0 1.0 0.0 0 0)))

(event EventBeginPlay
  (Collision|AssignOnComponentBeginOverlap (delegate Custom|OnComponentBeginOverlap_Event)))

(event EventTick
  (params (DeltaSeconds :type Float%20%28single-precision%29)))