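; B_Discharge_Simulation is an actor that repeatedly launches B_Projectile actors along its Arrow component, simulating discharge fire.
; BeginPlay starts a looping timer that calls Fire every second.
; Fire spawns a projectile at the Arrow transform and pushes its static mesh with a mass-independent force along the arrow's forward vector, much stronger when the Supersonic flag is set.
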(event Custom|Fire
  (bind _returnvalue (Game|SpawnActorfromClass "/ALSXT/ALS/Blueprints/B_Projectile.B_Projectile_C" (Transformation|GetWorldTransform (Variables|Default|GetArrow)) "AlwaysSpawn" 0 0))
  (Physics|AddForce (Variables|/ALSXT/ALS/Blueprints/B_Projectile.B_Projectile_C|GetStaticMesh _returnvalue) (* (Math|Vector|GetForwardVector (Variables|Default|GetArrow)) (select (Variables|Default|GetSupersonic) 5e+05 1e+05)) "None" true))

(event EventBeginPlay
  (Utilities|Time|SetTimerbyFunctionName 0 "Fire" 1.0 true))

(event Collision|EventActorBeginOverlap
  (params (OtherActor :type Actor%20Object%20Reference)))

(event EventTick
  (params (DeltaSeconds :type Float%20%28single-precision%29)))

(fn ConstructionScript)