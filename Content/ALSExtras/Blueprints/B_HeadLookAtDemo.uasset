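; Demo actor for ALSXT head look-at, with a constantly rotating static mesh inside a trigger sphere.
; On overlap, it enables an ALSXT character's head look-at at the mesh location if that world position dotted with the character mesh's forward vector is negative.
; Ending the overlap disables look-at.
; The look-at query functions are stubs returning defaults.
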(event OnComponentBeginOverlap(Sphere)
  (params (OverlappedComponent :type Primitive%20Component%20Object%20Reference) (OtherActor :type Actor%20Object%20Reference) (OtherComp :type Primitive%20Component%20Object%20Reference) (OtherBodyIndex :type Integer) (bFromSweep :type Boolean) (SweepResult :type Hit%20Result%20Structure%20%28by%20ref%29))
  (bind _staticmesh (Variables|Default|GetStaticMesh))
  (bind _returnvalue (Transformation|GetWorldLocation _staticmesh))
  (bind _asalsxtcharacter (Utilities|Casting|CastToALSXTCharacter OtherActor))
  (if (< (Math|Vector|DotProduct _returnvalue (Math|Vector|GetForwardVector (Variables|/Script/Engine.Character|GetMesh _asalsxtcharacter))) 0.0)
    (Class|ALSXTCharacter|SetHeadLookatState _asalsxtcharacter (Utilities|Struct|MakeALSXTHeadLookAtState true 0 _returnvalue))))

(event OnComponentEndOverlap(Sphere)
  (params (OverlappedComponent :type Primitive%20Component%20Object%20Reference) (OtherActor :type Actor%20Object%20Reference) (OtherComp :type Primitive%20Component%20Object%20Reference) (OtherBodyIndex :type Integer))
  (bind _asalsxtcharacter (Utilities|Casting|CastToALSXTCharacter OtherActor))
  (Class|ALSXTCharacter|SetHeadLookatState _asalsxtcharacter (Utilities|Struct|MakeALSXTHeadLookAtState false)))

(event EventBeginPlay)

(event Collision|EventActorBeginOverlap
  (params (OtherActor :type Actor%20Object%20Reference)))

(event EventTick
  (params (DeltaSeconds :type Float%20%28single-precision%29))
  (Transformation|AddWorldRotation (Variables|Default|GetStaticMesh) "0.000000,0.100000,0.100000" false false))

(fn ConstructionScript)

(fn CanbeHeadLookedat
  (return false))

(fn CanHeadLookat
  (return false))

(fn GetFacialReactions
  (return ""))

(fn GetHeadLookatLocation
  (return "0, 0, 0"))

(fn GetRating
  (return 0.0))

(fn IsinFrontOf
  (params (LookAtActorLocation :type Vector :default "0, 0, 0"))
  (return false))