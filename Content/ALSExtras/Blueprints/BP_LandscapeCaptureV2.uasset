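; Landscape capture actor that centers an orthographic scene capture over the level's Landscape, sizes it to the landscape bounds and captures once on BeginPlay.
; BeginPlay also publishes capture size to MPC_Capture and clears both render targets.
; Tick publishes capture location and draws M_DrawToPersistent into a render target using a normalized move offset.
; Pixel-snapped movement, water/landscape capture filtering and DrawBrush's canvas drawing are disconnected.
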(event EventBeginPlay
  (bind _returnvalue (Actor|GetActorOfClass "/Script/Landscape.Landscape"))
  (bind _output_get (Variables|Default|SetLandscape _returnvalue))
  (Transformation|SetActorLocation (Math|Vector|MakeVector (.X (Math|Vector|BreakVector (.Origin (Collision|GetActorBounds _output_get false false)))) (.Y (Math|Vector|BreakVector (.Origin (Collision|GetActorBounds _output_get false false)))) (.z (Transformation|GetActorLocation))) false true)
  (Transformation|SetMobility (Variables|Default|GetSceneCaptureComponent2D) "Static")
  (Variables|/Script/Engine.SceneCaptureComponent2D|SetOrthoWidth (Variables|DecalActor|GetCaptureComponent2D) (.x (* (.BoxExtent (Collision|GetActorBounds _output_get false false)) 2.0)))
  (Rendering|Material|SetScalarParameterValue "/ALSXT/ALSExtras/Materials/Terrain/MPC_Capture.MPC_Capture" "CaptureSize" (Variables|/Script/Engine.SceneCaptureComponent2D|GetOrthoWidth (Variables|DecalActor|GetCaptureComponent2D)) :!class /Script/Engine.KismetMaterialLibrary)
  (bind _returnvalue_2 (Rendering|Material|CreateDynamicMaterialInstance "/ALSXT/ALSExtras/Materials/Terrain/M_DrawToPersistent.M_DrawToPersistent" "None" "None" :!class /Script/Engine.KismetMaterialLibrary))
  (Variables|Default|SetDrawMaterial _returnvalue_2)
  (Rendering|ClearRenderTarget2D "/ALSXT/ALSExtras/Materials/RenderTargets/RT_LandscapeCapture.RT_LandscapeCapture")
  (Rendering|ClearRenderTarget2D "/ALSXT/ALSExtras/Materials/RenderTargets/RT_LandscapeCapturePersistent.RT_LandscapeCapturePersistent")
  (Rendering|SceneCapture|CaptureScene (Variables|Default|GetSceneCaptureComponent2D) :!class /Script/Engine.SceneCaptureComponent2D))

(event EventTick
  (params (DeltaSeconds :type Float%20%28single-precision%29))
  (CallFunction|MoveCapture)
  (CallFunction|DrawtoPersistent))

(fn ConstructionScript)

(fn DrawtoPersistent
  (bind _capturecomponent2d (Variables|DecalActor|GetCaptureComponent2D))
  (bind _moveoffset (Variables|Default|GetMoveOffset))
  (bind _orthowidth (Variables|/Script/Engine.SceneCaptureComponent2D|GetOrthoWidth _capturecomponent2d))
  (bind _returnvalue (/ _moveoffset _orthowidth))
  (Rendering|Material|SetVectorParameterValue (Variables|Default|GetDrawMaterial) "Offset" (Utilities|Struct|MakeLinearColor (.x _returnvalue) (.y _returnvalue) 0.0 1.0) :!class /Script/Engine.MaterialInstanceDynamic)
  (Rendering|DrawMaterialtoRenderTarget (Variables|Default|GetRenderTarget) (Variables|Default|GetDrawMaterial)))

(fn MoveCapture
  (Rendering|Material|SetVectorParameterValue "/ALSXT/ALSExtras/Materials/Terrain/MPC_Capture.MPC_Capture" "CaptureLocation" (Math|Conversions|ToLinearColor(Vector) (Transformation|GetActorLocation)) :!class /Script/Engine.KismetMaterialLibrary)
  (return))

(fn DrawBrush
  (params (BrushTexture :type Texture%202D%20Object%20Reference) (BrushSize :type Float%20%28double-precision%29) (DrawLocation :type Vector%202D%20Structure) (Rotation :type Float%20%28double-precision%29))
  (bind _brushmaterial (Variables|Default|GetBrushMaterial))
  (Utilities|FlowControl|Sequence
    (:then_0
      (Rendering|Material|SetTextureParameterValue _brushmaterial "BrushTexture" BrushTexture)
      (Rendering|Material|SetTextureParameterValue _brushmaterial "Texture" BrushTexture))))