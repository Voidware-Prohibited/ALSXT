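; B_Ladder is a spline-driven ladder actor for levels, built procedurally in the construction script with no active runtime logic.
; Spline mesh components follow the spline point to point to form the ladder body, and a static mesh caps its end.
; Static mesh rungs repeat at RungDistance intervals along the spline length, each taking the spline's local transform at that distance.
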(event EventBeginPlay)

(event Collision|EventActorBeginOverlap
  (params (OtherActor :type Actor%20Object%20Reference)))

(event EventTick
  (params (DeltaSeconds :type Float%20%28single-precision%29)))

(fn ConstructionScript
  (bind _spline (Variables|Default|GetSpline))
  (bind _spline_2 (Variables|Default|GetSpline))
  (Utilities|FlowControl|Sequence
    (:then_0
      (AddComponent|AddStaticMeshComponent false (Math|Transform|MakeTransform (Spline|GetLocationatSplinePoint (Variables|Default|GetSpline) (Spline|GetNumberOfSplinePoints (Variables|Default|GetSpline)) "Local"))))
    (:then_1
      (for _index (range 0 (Spline|GetNumberOfSplinePoints (Variables|Default|GetSpline)))
        (bind _returnvalue (AddComponent|AddSplineMeshComponent false (Math|Transform|MakeTransform "0, 0, 0" "0.000000,45.000000,0.000000")))
        (SplineMesh|SetStartandEnd _returnvalue (Spline|GetLocationatSplinePoint _spline _index "Local") (Spline|GetTangentatSplinePoint _spline _index "Local") (Spline|GetLocationatSplinePoint _spline_2 (+ _index 1) "Local") (Spline|GetTangentatSplinePoint _spline_2 (+ _index 1) "Local") true :!class /Script/Engine.SplineMeshComponent)))
    (:then_2
      (for _index_2 (range 0 (.ReturnValue (Math|Float|Division(WholeandRemainder) (Spline|GetSplineLength (Variables|Default|GetSpline)) (Variables|Default|GetRung%20Distance))))
        (AddComponent|AddStaticMeshComponent false (Spline|GetTransformatDistanceAlongSpline (Variables|Default|GetSpline) (* (Variables|Default|GetRung%20Distance) _index_2) "Local" false))))))