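; B_ExplosionSim is a level actor that simulates a repeating explosion, started by a looping timer only on non-authority instances.
; Each Explode spawns a Niagara effect with sound and attaches a temporary sphere collision, destroyed when the effect finishes.
; Overlapping components receive a radial impulse, and overlapping ALS characters also ragdoll with an impulse on their mesh.
; Begin-overlap and hit handlers exist, but their binding is disconnected.
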(event Custom|Explode
  (bind _returnvalue (Niagara|SpawnSystematLocation "/ALSXT/ALSExtras/Particles/N_Explosion.N_Explosion" (Transformation|GetWorldLocation (Variables|Default|GetDefaultSceneRoot))))
  (Variables|Default|SetNiagara _returnvalue)
  (bind _returnvalue_2 (AddComponent|AddSphereComponent true))
  (bind _output_get (Variables|Default|SetSphere%20Collision _returnvalue_2))
  (Transformation|AttachComponentToComponent _output_get (Variables|Default|GetNiagara) "None" "KeepRelative" "KeepRelative" "KeepRelative" true)
  (Audio|PlaySoundatLocation "/ALSXT/ALSExtras/Audio/Hazards/Explosion02.Explosion02" (Transformation|GetWorldLocation (Variables|Default|GetNiagara)) "0, 0, 0" 1.0 1.0 0.0 "/ALS/ALS/Audio/Footsteps/SA_Als_Footstep.SA_Als_Footstep" 0 0 0)
  (CallFunction|ApplyForce)
  (EventDispatchers|AssignOnSystemFinished (Variables|Default|GetNiagara) (delegate Custom|OnSystemFinished_Event)))

(event Custom|OnComponentBeginOverlap_Event_0
  (params (OverlappedComponent :type Primitive%20Component%20Object%20Reference) (OtherActor :type Actor%20Object%20Reference) (OtherComp :type Primitive%20Component%20Object%20Reference) (OtherBodyIndex :type Integer) (bFromSweep :type Boolean) (SweepResult :type Hit%20Result%20Structure%20%28by%20ref%29))
  (bind _asals_character (Utilities|Casting|CastToAlsCharacter OtherActor)
    (:then
      (Class|AlsCharacter|StartRagdolling _asals_character)
      (Physics|AddRadialImpulse (Variables|/Script/Engine.Character|GetMesh _asals_character) (Transformation|GetWorldLocation (Variables|Default|GetNiagara)) 8e+01 1e+05 "RIF_Linear" false))
    (:CastFailed
      (Physics|AddRadialImpulse OtherComp (Transformation|GetWorldLocation (Variables|Default|GetNiagara)) 3e+02 1e+05 "RIF_Constant" false))))

(event Custom|OnSystemFinished_Event
  (params (PSystem :type Niagara%20Component%20Object%20Reference))
  (bind _sphere_collision (Variables|Default|GetSphere%20Collision)
    (:then
      (Components|DestroyComponent _sphere_collision))
    (:else)))

(event Custom|OnComponentHit_Event
  (params (HitComponent :type Primitive%20Component%20Object%20Reference) (OtherActor :type Actor%20Object%20Reference) (OtherComp :type Primitive%20Component%20Object%20Reference) (NormalImpulse :type Vector) (Hit :type Hit%20Result%20Structure%20%28by%20ref%29))
  (bind _asals_character (Utilities|Casting|CastToAlsCharacter OtherActor)
    (:then
      (Class|AlsCharacter|StartRagdolling _asals_character)
      (Physics|AddRadialImpulse (Variables|/Script/Engine.Character|GetMesh _asals_character) (Transformation|GetWorldLocation (Variables|Default|GetNiagara)) 8e+01 1e+05 "RIF_Linear" false))
    (:CastFailed
      (Physics|AddRadialImpulse OtherComp (Transformation|GetWorldLocation (Variables|Default|GetNiagara)) 3e+02 1e+05 "RIF_Constant" false))))

(event Custom|Apply%20Force%20To%20Overlapping%20Actors
  (for _array_element (Collision|GetOverlappingActors (Variables|Default|GetSphere%20Collision) 0 :!class /Script/Engine.PrimitiveComponent)
    (bind _asals_character (Utilities|Casting|CastToAlsCharacter _array_element))
    (Class|AlsCharacter|StartRagdolling _asals_character)
    (Physics|AddRadialImpulse (Variables|/Script/Engine.Character|GetMesh _asals_character) (Transformation|GetWorldLocation (Variables|Default|GetNiagara)) 3e+02 1e+06 "RIF_Linear" false)))

(event Custom|Apply%20Force%20To%20Overlapping%20Components
  (for _array_element (Class|PrimitiveComponent|GetOverlappingComponents (Variables|Default|GetSphere%20Collision))
    (Physics|AddRadialImpulse _array_element (Transformation|GetWorldLocation (Variables|Default|GetNiagara)) 3e+02 1e+06 "RIF_Linear" false)))

(event Custom|Apply%20Force
  (CallFunction|ApplyForcetoOverlappingActors)
  (CallFunction|ApplyForcetoOverlappingComponents))

(event EventBeginPlay
  (Networking|SwitchHasAuthority
    (:Remote
      (Utilities|Time|SetTimerbyFunctionName 0 "Explode" 1.0 true))))

(event Collision|EventActorBeginOverlap
  (params (OtherActor :type Actor%20Object%20Reference)))

(event EventTick
  (params (DeltaSeconds :type Float%20%28single-precision%29)))

(fn ConstructionScript)